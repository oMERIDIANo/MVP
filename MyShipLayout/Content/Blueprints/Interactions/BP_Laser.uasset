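; BP_Laser is a pickup actor for the Laser Cutter tool that the player collects to gain a laser.
; Overlapping its Box component prints a pickup prompt on screen while the tool has not been picked up.
; Its Interact function sets the FoundTool flag on the player's ThirdPersonCharacter, destroys the actor and prints a hint for shooting the laser.
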(event OnComponentBeginOverlap(Box)
  (params (OverlappedComponent :type Primitive%20Component%20Object%20Reference) (OtherActor :type Actor%20Object%20Reference) (OtherComp :type Primitive%20Component%20Object%20Reference) (OtherBodyIndex :type Integer) (bFromSweep :type Boolean) (SweepResult :type Hit%20Result%20Structure%20%28by%20ref%29))
  (if (not (Variables|Default|GetpickedUpTool?))
    (Development|PrintString "Press E to pickup Laser Cutter" true true "(R=1.000000,G=1.000000,B=1.000000,A=1.000000)" 4.0)))

(event EventBeginPlay)

(event Collision|EventActorBeginOverlap
  (params (OtherActor :type Actor%20Object%20Reference)))

(event EventTick
  (params (DeltaSeconds :type Float%20%28single-precision%29)))

(fn ConstructionScript)

(fn Interact
  (Variables|Default|SetpickedUpTool? true)
  (bind _asthird_person_character (Utilities|Casting|CastToThirdPersonCharacter (Game|GetPlayerCharacter 0)))
  (bind _output_get (Variables|/Game/Blueprints/Character/ThirdPersonCharacter.ThirdPersonCharacter_C|SetfoundTool? _asthird_person_character true))
  (Actor|DestroyActor)
  (Development|PrintString "Left Click Mouse to shoot laser" true true "(R=1.000000,G=1.000000,B=1.000000,A=1.000000)" 5.0)
  (return _output_get))