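; BP_EmergencyLights is an emergency light whose spotlight depends on two switch actors, BP_EMLS1 and BP_EMLS2, both being on.
; BeginPlay sets the spotlight's initial visibility from both switch states.
; SwitchLight rechecks them and, only when both are on, shows the light, plays a quiet electricity sound and calls Test.
; SwitchLight has no branch that turns the light off.
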(event EventBeginPlay
  (bind _asbp_emls1 (Utilities|Casting|CastToBP_EMLS1 (Variables|Default|GetSwitchActor1)))
  (bind _asbp_emls2 (Utilities|Casting|CastToBP_EMLS2 (Variables|Default|GetSwitchActor2)))
  (Rendering|SetVisibility (Variables|Default|GetSpotLight) (and (Variables|/Game/Blueprints/Interactions/BP_EMLS2.BP_EMLS2_C|GetisOn? _asbp_emls2) (Variables|/Game/Blueprints/Interactions/BP_EMLS1.BP_EMLS1_C|GetisOn? _asbp_emls1)) false))

(fn ConstructionScript)

(fn SwitchLight
  (bind _asbp_emls1 (Utilities|Casting|CastToBP_EMLS1 (Variables|Default|GetSwitchActor1)))
  (bind _asbp_emls2 (Utilities|Casting|CastToBP_EMLS2 (Variables|Default|GetSwitchActor2)))
  (if (and (Variables|/Game/Blueprints/Interactions/BP_EMLS2.BP_EMLS2_C|GetisOn? _asbp_emls2) (Variables|/Game/Blueprints/Interactions/BP_EMLS1.BP_EMLS1_C|GetisOn? _asbp_emls1))
    (Rendering|SetVisibility (Variables|Default|GetSpotLight) (and (Variables|/Game/Blueprints/Interactions/BP_EMLS2.BP_EMLS2_C|GetisOn? _asbp_emls2) (Variables|/Game/Blueprints/Interactions/BP_EMLS1.BP_EMLS1_C|GetisOn? _asbp_emls1)) false)
    (Audio|PlaySoundatLocation "/Game/Blueprints/Interactions/Electricity.Electricity" "0, 0, 0" "0, 0, 0" 0.1 1.0 0.5 0 0 0)
    (Default|CallTest)))