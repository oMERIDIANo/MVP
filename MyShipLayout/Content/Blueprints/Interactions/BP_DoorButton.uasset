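; BP_DoorButton is an interactable button that toggles a door open and closed when Interact is pressed.
; Player overlap with InteractCollider enables input and opens a Gate, while any overlap prints a control prompt.
; A press plays sounds at world origin, then passes the Gate into the ButtonPressAnim timeline macro, whose finish drives a FlipFlop playing or reversing the door-sliding timeline.
; The construction script positions the button from ButtonTransform.
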(event OnComponentBeginOverlap(InteractCollider)
  (params (OverlappedComponent :type Primitive%20Component%20Object%20Reference) (OtherActor :type Actor%20Object%20Reference) (OtherComp :type Primitive%20Component%20Object%20Reference) (OtherBodyIndex :type Integer) (bFromSweep :type Boolean) (SweepResult :type Hit%20Result%20Structure%20%28by%20ref%29))
  ;[1 1 1] Button/Door Interaction
  (Development|PrintString "Press E to Interact : Press F for Flashlight" true true "(R=1.000000,G=1.000000,B=1.000000,A=1.000000)" 4.0)
  (Audio|PlaySoundatLocation "/Game/Audio/UIPopup1.UIPopup1" "0, 0, 0" "0, 0, 0" 1.0 1.0 0.0 0 0 0)
  (Utilities|Casting|CastToThirdPersonCharacter OtherActor)
  (Input|EnableInput (Game|GetPlayerController 0))
  (Utilities|FlowControl|Gate true) ; enters at Open
)

(event OnComponentEndOverlap(InteractCollider)
  (params (OverlappedComponent :type Primitive%20Component%20Object%20Reference) (OtherActor :type Actor%20Object%20Reference) (OtherComp :type Primitive%20Component%20Object%20Reference) (OtherBodyIndex :type Integer))
  ;[1 1 1] Button/Door Interaction
  (Utilities|Casting|CastToThirdPersonCharacter OtherActor)
  (Input|DisableInput (Game|GetPlayerController 0))
  (Utilities|FlowControl|Gate true) ; enters at Close
)

(event Input|ActionEvents|InputActionInteract
  (params (Key :type Key%20Structure :default "None"))
  ;[1 1 1] Button/Door Interaction
  (:Pressed
    (Audio|PlaySoundatLocation "/Game/Audio/ComputerDoo.ComputerDoo" "0, 0, 0" "0, 0, 0" 1.0 1.0 0.0 0 0 0)
    (Audio|PlaySoundatLocation "/Game/Audio/DockDoor.DockDoor" "0, 0, 0" "0, 0, 0" 1.0 1.0 0.0 0 0 0)
    (Utilities|FlowControl|Gate true
      (:Exit
        (|ButtonPressAnim
          (:toFinish
            (Utilities|FlowControl|FlipFlop
              (:A
                (bind _newtrack_0 (Timeline|Timeline_1 Play)
                  (:Update
                    (Transformation|SetRelativeLocation (Variables|Default|GetDoor) (Math|Vector|Lerp(Vector) (Variables|Default|GetA) (Variables|Default|GetB) _newtrack_0) false false))))
              (:B
                (Timeline|Timeline_1 Reverse)))))))))

(fn ConstructionScript
  (Transformation|SetRelativeTransform (Variables|Default|GetButton) (Variables|Default|GetButton%20Transform) false false))

(fn Interact
  (return false))