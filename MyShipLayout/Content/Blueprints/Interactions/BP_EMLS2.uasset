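; BP_EMLS2 is an interactable switch that toggles the emergency lights and prints a message calling it a power panel when switched on.
; Interact plays a click at world origin, flips IsOn and calls SwitchLight on BP_EmergencyLights actors found with GetAllActorsOfClass.
; Switching on loops through every light before returning true, while the off branch wires that return inside its loop body, so it exits after the first light.
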(fn ConstructionScript)

(fn Interact
  (Audio|PlaySoundatLocation "/Game/Audio/ButtonClick.ButtonClick" "0, 0, 0" "0, 0, 0" 1.0 1.0 0.0 0 0 0)
  (if (not (Variables|Default|GetisOn?))
    (Variables|Default|SetisOn? true)
    (Development|PrintString "Switched on a power panel" true true "(R=1.000000,G=1.000000,B=1.000000,A=1.000000)" 3.0)
    (bind _outactors (Actor|GetAllActorsOfClass "/Game/Blueprints/Interactions/BP_EmergencyLights.BP_EmergencyLights_C"))
    (for _array_element _outactors
      (Default|SwitchLight _array_element))
    (return true)
    (elif (Math|Boolean|Equal(Boolean) (Variables|Default|GetisOn?) true)
      (Variables|Default|SetisOn? false)
      (bind _outactors_2 (Actor|GetAllActorsOfClass "/Game/Blueprints/Interactions/BP_EmergencyLights.BP_EmergencyLights_C"))
      (for _array_element_2 _outactors_2
        (Default|SwitchLight _array_element_2)
        (return true)))))